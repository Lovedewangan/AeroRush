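; BP_New_Environment is an environment segment actor that reacts to BP_Character through three trigger boxes and exposes an Arrow transform as the attach point for a new environment.
; Box plays a Timeline that adds one to BP_GameMode's CurrentPoints on every update, so points gained depend on update count.
; Box2 sets the character's gravity scale to a fixed value, and Box3 destroys the segment.
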(event `self.ReceiveActorBeginOverlap`
  (params (OtherActor :type "Actor Object Reference")))

(event `self.Box.OnComponentBeginOverlap`
  (params (OverlappedComponent :type "PrimitiveComponent Object Reference") (OtherActor :type "Actor Object Reference") (OtherComp :type "PrimitiveComponent Object Reference") (OtherBodyIndex :type Integer) (bFromSweep :type Boolean) (SweepResult :type "HitResult Structure (by ref)"))
  (cast `/Game/Asset/Blueprints/BP_Character` OtherActor)
  (`Timeline|Timeline`
    (:`Update`
      (bind _asbp_game_mode (cast `/Game/Asset/Blueprints/BP_GameMode` (`GameplayStatics.GetGameMode`)))
      (set `/Game/Asset/Blueprints/BP_GameMode.Current Points` (+ (`/Game/Asset/Blueprints/BP_GameMode.Current Points` _asbp_game_mode) 1) _asbp_game_mode))))

(event `self.Box2.OnComponentBeginOverlap`
  (params (OverlappedComponent :type "PrimitiveComponent Object Reference") (OtherActor :type "Actor Object Reference") (OtherComp :type "PrimitiveComponent Object Reference") (OtherBodyIndex :type Integer) (bFromSweep :type Boolean) (SweepResult :type "HitResult Structure (by ref)"))
  (bind _asbp_character (cast `/Game/Asset/Blueprints/BP_Character` OtherActor))
  (set `CharacterMovementComponent.GravityScale` 0.6 (`Character.CharacterMovement` _asbp_character)))

(event `self.Box3.OnComponentBeginOverlap`
  (params (OverlappedComponent :type "PrimitiveComponent Object Reference") (OtherActor :type "Actor Object Reference") (OtherComp :type "PrimitiveComponent Object Reference") (OtherBodyIndex :type Integer) (bFromSweep :type Boolean) (SweepResult :type "HitResult Structure (by ref)"))
  (cast `/Game/Asset/Blueprints/BP_Character` OtherActor)
  (`self.K2_DestroyActor`))

(fn `Get attach point New Environment`
  (returns (ReturnValue :type "Transform Structure"))
  (return (`SceneComponent.K2_GetComponentToWorld` (`self.Arrow`))))

(fn `NewFunction`)

(fn `UserConstructionScript`)