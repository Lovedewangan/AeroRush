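; BP_Player is a player Blueprint with keyboard-driven forward movement and lane snapping.
; Pressing W adds a single movement input along world X with a very large vector, rather than applying it every tick.
; A and D teleport the player to the location and rotation of the Lane0 and Lane2 references, then print a debug string.
; BeginPlay, Tick, overlap and the construction script are empty.
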(event `self.ReceiveBeginPlay`)

(event `self.ReceiveTick`
  (params (DeltaSeconds :type "Float (single-precision)")))

(event `Key|W`
  (params (Key :type "Key Structure"))
  (:`Pressed`
    (`self.AddMovementInput` (100000000.0 0.0 0.0))))

(event `Key|A`
  (params (Key :type "Key Structure"))
  (bind (_returnvalue_location _returnvalue_rotation) (`KismetMathLibrary.BreakTransform` (`self.GetTransform` (`self.Lane0`))))
  (:`Pressed`
    (`self.K2_SetActorLocationAndRotation` _returnvalue_location _returnvalue_rotation)
    (`KismetSystemLibrary.PrintString` "Hello")))

(event `Key|D`
  (params (Key :type "Key Structure"))
  (bind (_returnvalue_location _returnvalue_rotation) (`KismetMathLibrary.BreakTransform` (`self.GetTransform` (`self.Lane2`))))
  (:`Pressed`
    (`self.K2_SetActorLocationAndRotation` _returnvalue_location _returnvalue_rotation)
    (`KismetSystemLibrary.PrintString` "Hello")))

(fn `UserConstructionScript`)