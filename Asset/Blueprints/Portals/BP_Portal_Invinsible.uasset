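; Portal actor named for invincibility that launches the player character along a short transition when it overlaps the Sphere.
; The overlap plays a whoosh sound and a one-shot animation on the character mesh, then starts the Transition timeline.
; Each timeline update nudges the character by a fixed offset and adds a point to BP_GameMode, so both totals depend on frame rate.
; No invincibility state is set; the speed and camera nodes are unconnected.
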(event `self.Sphere.OnComponentBeginOverlap`
  (params (OverlappedComponent :type "PrimitiveComponent Object Reference") (OtherActor :type "Actor Object Reference") (OtherComp :type "PrimitiveComponent Object Reference") (OtherBodyIndex :type Integer) (bFromSweep :type Boolean) (SweepResult :type "HitResult Structure (by ref)"))
  (bind _asbp_character (cast `/Game/Asset/Blueprints/BP_Character` OtherActor))
  (`GameplayStatics.PlaySound2D` "/Game/Asset/Blueprints/whoop-sound-effect-320-kbps-ytmp3snet_KX7SSSQj.whoop-sound-effect-320-kbps-ytmp3snet_KX7SSSQj" 1.0 1.0 0.0 null null)
  (`SkeletalMeshComponent.PlayAnimation` (`Character.Mesh` _asbp_character) "/Game/Asset/Animation/New_Airplane_Animation/Invinsible/Invinsible_Animation.Invinsible_Animation" false)
  (`Timeline|Transition`
    (:`Update`
      (`self.K2_AddActorWorldTransform` _asbp_character (`KismetMathLibrary.MakeTransform` (0.0 -10.0 23.0)) false false)
      (bind _asbp_game_mode (cast `/Game/Asset/Blueprints/BP_GameMode` (`GameplayStatics.GetGameMode`)))
      (set `/Game/Asset/Blueprints/BP_GameMode.Current Points` (+ (`/Game/Asset/Blueprints/BP_GameMode.Current Points` _asbp_game_mode) 1) _asbp_game_mode))))

(event `self.Portal.OnComponentBeginOverlap`
  (params (OverlappedComponent :type "PrimitiveComponent Object Reference") (OtherActor :type "Actor Object Reference") (OtherComp :type "PrimitiveComponent Object Reference") (OtherBodyIndex :type Integer) (bFromSweep :type Boolean) (SweepResult :type "HitResult Structure (by ref)")))

(fn `UserConstructionScript`
  (`parent.UserConstructionScript`))