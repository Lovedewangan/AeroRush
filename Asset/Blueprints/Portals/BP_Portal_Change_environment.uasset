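; BP_Portal_Change_environment is a portal that launches BP_Character when it enters the portal's sphere.
; The overlap plays a timeline that each update shifts the character up and along negative Y, zeroes gravity and sets a very high walk speed, with no reset here.
; GetAttachPointNewEnvironment exposes the Arrow's world transform as an attach point.
; BP_Hallway spawning logic is present but unconnected, so it never runs.
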(event `self.Sphere.OnComponentBeginOverlap`
  (params (OverlappedComponent :type "PrimitiveComponent Object Reference") (OtherActor :type "Actor Object Reference") (OtherComp :type "PrimitiveComponent Object Reference") (OtherBodyIndex :type Integer) (bFromSweep :type Boolean) (SweepResult :type "HitResult Structure (by ref)"))
  (bind _asbp_character (cast `/Game/Asset/Blueprints/BP_Character` OtherActor))
  (`Timeline|Timeline`
    (:`Update`
      (`self.K2_AddActorWorldTransform` _asbp_character (`KismetMathLibrary.MakeTransform` (0.0 -100.0 217.0)) false false)
      (bind _charactermovement (`Character.CharacterMovement` _asbp_character))
      (set `CharacterMovementComponent.GravityScale` 0.0 _charactermovement)
      (set `CharacterMovementComponent.MaxWalkSpeed` 15000.0 _charactermovement))))

(fn `Get Attach Point New Environment`
  (returns (ReturnValue :type "Transform Structure"))
  (return (`SceneComponent.K2_GetComponentToWorld` (`self.Arrow`))))

(fn `UserConstructionScript`
  (`parent.UserConstructionScript`))