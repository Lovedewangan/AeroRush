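; Floor tile for an endless airplane runner that populates itself with obstacles, power-ups and coins.
; The construction script builds arrow-based spawn points along each lane, shuffles them and attaches random child actors.
; Power-ups appear only when the GameMode's FloorCount exceeds five, then reset that counter.
; Overlapping the Box tells BP_GameMode to extend the floor, raises the character's clamped speed and adds multiplier-scaled points.
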(event `self.ReceiveTick`
  (params (DeltaSeconds :type "Float (single-precision)")))

(event `self.Box.OnComponentBeginOverlap`
  (params (OverlappedComponent :type "PrimitiveComponent Object Reference") (OtherActor :type "Actor Object Reference") (OtherComp :type "PrimitiveComponent Object Reference") (OtherBodyIndex :type Integer) (bFromSweep :type Boolean) (SweepResult :type "HitResult Structure (by ref)"))
  ;[1 1 1] Extending Floor
  (bind _asbp_game_mode (cast `/Game/Asset/Blueprints/BP_GameMode` (`GameplayStatics.GetGameMode`)))
  (`/Game/Asset/Blueprints/BP_GameMode.Extend Floor` _asbp_game_mode)
  ;[1 1 1] Increasing Airplane speed
  (bind _asbp_character (cast `/Game/Asset/Blueprints/BP_Character` (`GameplayStatics.GetPlayerCharacter` 0)))
  (bind _charactermovement (`Character.CharacterMovement` _asbp_character))
  (set `CharacterMovementComponent.MaxWalkSpeed` (`KismetMathLibrary.FClamp` (* (`CharacterMovementComponent.MaxWalkSpeed` _charactermovement) 1.01) 5000.0 50000.0) _charactermovement)
  ;[1 1 1] Current Score
  (bind _asbp_game_mode_2 (cast `/Game/Asset/Blueprints/BP_GameMode` (`GameplayStatics.GetGameMode`)))
  (set `/Game/Asset/Blueprints/BP_GameMode.Current Points` (+ (* (`/Game/Asset/Blueprints/BP_GameMode.Points Multi` _asbp_game_mode_2) 5) (`/Game/Asset/Blueprints/BP_GameMode.Current Points` _asbp_game_mode_2)) _asbp_game_mode_2))

(fn `Coin Spawn Points`
  (for _array_element (`self.Lane Position`)
    (for _index (range 17)
      (bind _returnvalue (`AddComponent|NODE_AddArrowComponent-2` :`RelativeTransform` (`KismetMathLibrary.MakeTransform` (`KismetMathLibrary.MakeVector` _array_element (* _index 300.0)))))
      (`ArrowComponent.SetArrowColor` _returnvalue (struct :`R` 1.0 :`G` 0.997723 :`B` 0.858276 :`A` 1.0))
      (`KismetArrayLibrary.Array_Add` (`self.CSpawn Point`) (`SceneComponent.K2_GetComponentToWorld` _returnvalue)))))

(fn `Get Attach Point`
  (returns (ReturnValue :type "Transform Structure"))
  (return (`SceneComponent.K2_GetComponentToWorld` (`self.Arrow`))))

(fn `Setup Power Ups Spawn Points`
  (for _array_element (`self.Lane Position`)
    (for _index (range 2)
      (bind _returnvalue (`AddComponent|NODE_AddArrowComponent-1` :`RelativeTransform` (`KismetMathLibrary.MakeTransform` (`KismetMathLibrary.MakeVector` _array_element -4000.0))))
      (`KismetArrayLibrary.Array_Add` (`self.Spawn Points Power Ups`) (`SceneComponent.K2_GetComponentToWorld` _returnvalue)))))

(fn `Setup Spawn Points`
  (for _array_element (`self.Lane Position`)
    (for _index (range 2)
      (bind _returnvalue (`AddComponent|NODE_AddArrowComponent-0` :`RelativeTransform` (`KismetMathLibrary.MakeTransform` (`KismetMathLibrary.MakeVector` _array_element (* _index 0.0)))))
      (`KismetArrayLibrary.Array_Add` (`self.Spawn Points `) (`SceneComponent.K2_GetComponentToWorld` _returnvalue)))))

(fn `Spawn Coins`
  (locals (`Random Spawn Points` :type "Array of Transform Structure"))
  (bind _output_get (set `local.Random Spawn Points` (`self.CSpawn Point`)))
  (`KismetArrayLibrary.Array_Shuffle` _output_get)
  (for _index (range (+ (`KismetMathLibrary.RandomIntegerInRange` 8 14) 1))
    (switch `int` 0
      (:`0`
        (`AddComponent|NODE_AddChildActorComponent-15` :`RelativeTransform` (`KismetMathLibrary.MakeRelativeTransform` (`|GetArrayItem` (`local.Random Spawn Points`) _index) (`self.GetTransform`)))))))

(fn `Spawn Obstacles`
  (locals (`Random Spawn Points` :type "Array of Transform Structure"))
  (bind _output_get (set `local.Random Spawn Points` (`self.Spawn Points `)))
  (`KismetArrayLibrary.Array_Shuffle` _output_get)
  (for _index (range (+ (`KismetMathLibrary.RandomIntegerInRange` 0 1) 1))
    (switch `int` (`KismetMathLibrary.RandomIntegerInRange` 0 4)
      (:`0`
        (bind _returnvalue (`KismetMathLibrary.MakeRelativeTransform` (`|GetArrayItem` (`local.Random Spawn Points`) _index) (`self.GetTransform`)))
        (`AddComponent|NODE_AddChildActorComponent-2` :`RelativeTransform` _returnvalue))
      (:`1`
        (`AddComponent|NODE_AddChildActorComponent-3` :`RelativeTransform` _returnvalue))
      (:`2`
        (`AddComponent|NODE_AddChildActorComponent-4` :`RelativeTransform` _returnvalue))
      (:`3`
        (`AddComponent|NODE_AddChildActorComponent-5` :`RelativeTransform` _returnvalue))
      (:`4`
        (`AddComponent|NODE_AddChildActorComponent-6` :`RelativeTransform` _returnvalue)))))

(fn `Spawn Power Ups`
  (locals (`Random Spawn Points Power Ups` :type "Array of Transform Structure"))
  (bind _asbp_game_mode (cast `/Game/Asset/Blueprints/BP_GameMode` (`GameplayStatics.GetGameMode`)))
  (if (> (`/Game/Asset/Blueprints/BP_GameMode.Floor Count` _asbp_game_mode) 5)
    (bind _output_get (set `local.Random Spawn Points Power Ups` (`self.Spawn Points Power Ups`)))
    (`KismetArrayLibrary.Array_Shuffle` _output_get)
    (for _index (range (+ (`KismetMathLibrary.RandomIntegerInRange` 0) 1))
      (switch `int` (`KismetMathLibrary.RandomIntegerInRange` 0 1)
        (:`0`
          (bind _returnvalue (`KismetMathLibrary.MakeRelativeTransform` (`|GetArrayItem` (`local.Random Spawn Points Power Ups`) _index) (`self.GetTransform`)))
          (`AddComponent|NODE_AddChildActorComponent-7` :`RelativeTransform` _returnvalue))
        (:`1`
          (`AddComponent|NODE_AddChildActorComponent-8` :`RelativeTransform` _returnvalue)))
      (set `/Game/Asset/Blueprints/BP_GameMode.Floor Count` 0 _asbp_game_mode))))

(fn `UserConstructionScript`
  (`self.Setup Spawn Points`)
  (`self.Spawn Obstacles`)
  (`self.Setup Power Ups Spawn Points`)
  (`self.Spawn Power Ups`)
  (`self.Coin Spawn Points`)
  (`self.Spawn Coins`))