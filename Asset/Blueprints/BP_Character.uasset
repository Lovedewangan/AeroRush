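; Player character for a three-lane endless runner that moves forward automatically every Tick.
; Enhanced Input plays animations and triggers lane changes, which a timeline lerps along X between clamped lane positions, or a jump.
; BeginPlay shows the gameplay UI and adds the input mapping.
; Death disables movement and input, shows game over, then saves the high score if beaten and the GameMode's coin count to separate save slots.
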(event `self.ReceiveBeginPlay`
  ;[1 1 1] Input Mapping
  (bind _returnvalue (`|CreateWidget` "/Game/Asset/Blueprints/HUD/Gameplay_UI.Gameplay_UI_C"))
  (`UserWidget.AddToViewport` _returnvalue 0)
  (bind _asplayer_controller (cast `PlayerController` (`self.GetController`)))
  (bind _returnvalue_2 (pcsubsystem `EnhancedInputLocalPlayerSubsystem` _asplayer_controller))
  (`/Engine/EditorBlueprintResources/StandardMacros.IsValid` _returnvalue_2
    (:`Is Valid`
      (`EnhancedInputSubsystemInterface.AddMappingContext` _returnvalue_2 "/Game/Asset/Blueprints/Input/IMC_Airplane_Default.IMC_Airplane_Default" 0 (struct)))))

(event `self.ReceiveTick`
  (params (DeltaSeconds :type "Float (single-precision)"))
  ;[1 1 1] Infinite Run
  (`self.AddMovementInput` (0.0 -500.0 0.0) 1.0 true))

(event `Key|A`
  (params (Key :type "Key Structure")))

(event `Change Lanes`
  (params (`Shift Lanes` :type Integer))
  ;[1 1 1] Change Lane
  (set `self.Target Lane Index` (`KismetMathLibrary.Clamp` (+ `Shift Lanes` (`self.Current Lane Index`)) 0 2))
  (set `self.Current Y position` (.x (`self.K2_GetActorLocation`)))
  (bind (_direction _change_lane) (`Timeline|Transition` :!via `PlayFromStart`)
    (:`Update`
      (`self.K2_SetActorLocation` (`KismetMathLibrary.MakeVector` (`KismetMathLibrary.Lerp` (`self.Current Y position`) (`|GetArrayItem` (`self.Lane Position`) (`self.Target Lane Index`)) _change_lane) (.y (`self.K2_GetActorLocation`)) (.z (`self.K2_GetActorLocation`)))))
    (:`Finished`
      (set `self.Current Lane Index` (`self.Target Lane Index`)))))

(event `EnhancedInput|/Game/Asset/Blueprints/Input/Left_IA`
  (params (ActionValue :type "Vector2D Structure") (ElapsedSeconds :type "Float (double-precision)") (TriggeredSeconds :type "Float (double-precision)") (InputAction :type "InputAction Object Reference" :default "/Game/Asset/Blueprints/Input/Left_IA.Left_IA"))
  ;[1 1 1] Change Lane
  (:`Triggered`
    (`SkeletalMeshComponent.PlayAnimation` (`self.Mesh`) "/Game/Asset/Animation/New_Airplane_Animation/Left/Left_Anim.Left_Anim" false)
    (`self.Change Lanes` -1)))

(event `EnhancedInput|/Game/Asset/Blueprints/Input/Right_IA`
  (params (ActionValue :type "Vector2D Structure") (ElapsedSeconds :type "Float (double-precision)") (TriggeredSeconds :type "Float (double-precision)") (InputAction :type "InputAction Object Reference" :default "/Game/Asset/Blueprints/Input/Right_IA.Right_IA"))
  ;[1 1 1] Change Lane
  (:`Triggered`
    (`SkeletalMeshComponent.PlayAnimation` (`self.Mesh`) "/Game/Asset/Animation/New_Airplane_Animation/Right/Right_Anim.Right_Anim" false)
    (`self.Change Lanes` 1)))

(event `Key|D`
  (params (Key :type "Key Structure")))

(event `EnhancedInput|/Game/Asset/Blueprints/Input/Elevate_IA`
  (params (ActionValue :type "Vector2D Structure") (ElapsedSeconds :type "Float (double-precision)") (TriggeredSeconds :type "Float (double-precision)") (InputAction :type "InputAction Object Reference" :default "/Game/Asset/Blueprints/Input/Elevate_IA.Elevate_IA"))
  ;[1 1 1] Change Lane
  (:`Started`
    (`self.Elevate`)))

(event `Elevate`
  ;[1 1 1] Change Lane
  (`SkeletalMeshComponent.PlayAnimation` (`self.Mesh`) "/Game/Asset/Animation/New_Airplane_Animation/Jump/Jump_Animation.Jump_Animation" false)
  (`self.Jump`))

(fn `Death`
  (`CharacterMovementComponent.DisableMovement` (`self.CharacterMovement`))
  (`self.DisableInput` null)
  (`WidgetLayoutLibrary.RemoveAllWidgets`)
  (bind _returnvalue (`|CreateWidget` "/Game/Asset/Blueprints/HUD/GameOver_UI.GameOver_UI_C"))
  (`UserWidget.AddToViewport` _returnvalue 0)
  (set `PlayerController.bShowMouseCursor` true (`GameplayStatics.GetPlayerController` 0))
  (`self.SaveHighScore`)
  (`self.UpdateCoins`))

(fn `SaveHighScore`
  (bind _asbp_game_mode (cast `/Game/Asset/Blueprints/BP_GameMode` (`GameplayStatics.GetGameMode`)))
  (bind _returnvalue (`GameplayStatics.DoesSaveGameExist` "HighScoreValue"))
  (if _returnvalue
    (bind _returnvalue_2 (`GameplayStatics.LoadGameFromSlot` "HighScoreValue"))
    (bind _output_get (set `self.Saver Sub Class` _returnvalue_2))
    (bind _asrunner_save_game (cast `/Game/Asset/Blueprints/Runner_Save_Game` _output_get))
    (bind _current_points (`/Game/Asset/Blueprints/BP_GameMode.Current Points` _asbp_game_mode))
    (if (> _current_points (`/Game/Asset/Blueprints/Runner_Save_Game.HighScoreValue` _asrunner_save_game))
      (set `/Game/Asset/Blueprints/Runner_Save_Game.HighScoreValue` _current_points _asrunner_save_game)
      (`GameplayStatics.SaveGameToSlot` (`self.Saver Sub Class`) "HighScoreValue"))
    (else
      (bind _returnvalue_3 (`GameplayStatics.CreateSaveGameObject` "/Game/Asset/Blueprints/Runner_Save_Game.Runner_Save_Game_C"))
      (bind _output_get_2 (set `self.Saver Sub Class` _returnvalue_3))
      (bind _asrunner_save_game_2 (cast `/Game/Asset/Blueprints/Runner_Save_Game` _output_get_2))
      (set `/Game/Asset/Blueprints/Runner_Save_Game.HighScoreValue` _current_points _asrunner_save_game_2)
      (`GameplayStatics.SaveGameToSlot` (`self.Saver Sub Class`) "HighScoreValue"))))

(fn `UpdateCoins`
  (bind _asbp_game_mode (cast `/Game/Asset/Blueprints/BP_GameMode` (`GameplayStatics.GetGameMode`)))
  (bind _returnvalue (`GameplayStatics.DoesSaveGameExist` "CoinValue"))
  (if _returnvalue
    (bind _returnvalue_2 (`GameplayStatics.LoadGameFromSlot` "CoinValue"))
    (bind _output_get (set `self.Saver Sub Class` _returnvalue_2))
    (bind _asrunner_save_game (cast `/Game/Asset/Blueprints/Runner_Save_Game` _output_get))
    (bind _coins (`/Game/Asset/Blueprints/BP_GameMode.Coins` _asbp_game_mode))
    (set `/Game/Asset/Blueprints/Runner_Save_Game.CoinValue` _coins _asrunner_save_game)
    (`GameplayStatics.SaveGameToSlot` (`self.Saver Sub Class`) "CoinValue")
    (else
      (bind _returnvalue_3 (`GameplayStatics.CreateSaveGameObject` "/Game/Asset/Blueprints/Runner_Save_Game.Runner_Save_Game_C"))
      (bind _output_get_2 (set `self.Saver Sub Class` _returnvalue_3))
      (bind _asrunner_save_game_2 (cast `/Game/Asset/Blueprints/Runner_Save_Game` _output_get_2))
      (set `/Game/Asset/Blueprints/Runner_Save_Game.CoinValue` _coins _asrunner_save_game_2)
      (`GameplayStatics.SaveGameToSlot` (`self.Saver Sub Class`) "CoinValue"))))

(fn `UserConstructionScript`)