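; BP_Hallway is a high-speed hallway segment that fills itself with coins and exposes an arrow transform as an attach point.
; Its construction script builds arrow-marked spawn points along each lane, shuffles them and adds child actors at a random number of them.
; Three trigger boxes act on BP_Character: the first boosts speed, starts an effect, shifts the camera and ticks up GameMode points through timelines.
; The second reverses speed and camera; the third stops the effect and destroys the hallway.
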(event `self.ReceiveActorBeginOverlap`
  (params (OtherActor :type "Actor Object Reference")))

(event `self.Box.OnComponentBeginOverlap`
  (params (OverlappedComponent :type "PrimitiveComponent Object Reference") (OtherActor :type "Actor Object Reference") (OtherComp :type "PrimitiveComponent Object Reference") (OtherBodyIndex :type Integer) (bFromSweep :type Boolean) (SweepResult :type "HitResult Structure (by ref)"))
  (bind _asbp_character (cast `/Game/Asset/Blueprints/BP_Character` OtherActor))
  (`ActorComponent.Activate` (`/Game/Asset/Blueprints/BP_Character.NS_Moving_Effect` _asbp_character) false)
  (bind _charactermovement (`Character.CharacterMovement` _asbp_character))
  (set `CharacterMovementComponent.MaxWalkSpeed` (+ (`CharacterMovementComponent.MaxWalkSpeed` _charactermovement) 12000.0) _charactermovement)
  (`Timeline|Transition`
    (:`Update`
      (bind _camera (`/Game/Asset/Blueprints/BP_Character.Camera` _asbp_character))
      (bind (_returnvalue_x _returnvalue_y _returnvalue_z) (`KismetMathLibrary.BreakVector` (`SceneComponent.K2_GetComponentLocation` _camera)))
      (`SceneComponent.K2_SetWorldLocationAndRotation` _camera (`KismetMathLibrary.MakeVector` _returnvalue_x (+ _returnvalue_y 1.0) (- _returnvalue_z 0.4)) (struct :`Pitch` 2.0 :`Yaw` -90.0) false false)
      (`Timeline|Timeline`
        (:`Update`
          (bind _asbp_game_mode (cast `/Game/Asset/Blueprints/BP_GameMode` (`GameplayStatics.GetGameMode`)))
          (set `/Game/Asset/Blueprints/BP_GameMode.Current Points` (+ (`/Game/Asset/Blueprints/BP_GameMode.Current Points` _asbp_game_mode) 1) _asbp_game_mode))))))

(event `self.Box2.OnComponentBeginOverlap`
  (params (OverlappedComponent :type "PrimitiveComponent Object Reference") (OtherActor :type "Actor Object Reference") (OtherComp :type "PrimitiveComponent Object Reference") (OtherBodyIndex :type Integer) (bFromSweep :type Boolean) (SweepResult :type "HitResult Structure (by ref)"))
  (bind _asbp_character (cast `/Game/Asset/Blueprints/BP_Character` OtherActor))
  (bind _charactermovement (`Character.CharacterMovement` _asbp_character))
  (set `CharacterMovementComponent.MaxWalkSpeed` (- (`CharacterMovementComponent.MaxWalkSpeed` _charactermovement) 12000.0) _charactermovement)
  (`Timeline|Timeline_0`
    (:`Update`
      (bind _camera (`/Game/Asset/Blueprints/BP_Character.Camera` _asbp_character))
      (bind (_returnvalue_x _returnvalue_y _returnvalue_z) (`KismetMathLibrary.BreakVector` (`SceneComponent.K2_GetComponentLocation` _camera)))
      (`SceneComponent.K2_SetWorldLocationAndRotation` _camera (`KismetMathLibrary.MakeVector` _returnvalue_x (- _returnvalue_y 1.0) (+ _returnvalue_z 0.4)) (struct :`Pitch` -10.0 :`Yaw` -90.0) false false))))

(event `self.Box3.OnComponentBeginOverlap`
  (params (OverlappedComponent :type "PrimitiveComponent Object Reference") (OtherActor :type "Actor Object Reference") (OtherComp :type "PrimitiveComponent Object Reference") (OtherBodyIndex :type Integer) (bFromSweep :type Boolean) (SweepResult :type "HitResult Structure (by ref)"))
  (bind _asbp_character (cast `/Game/Asset/Blueprints/BP_Character` OtherActor))
  (`ActorComponent.Deactivate` (`/Game/Asset/Blueprints/BP_Character.NS_Moving_Effect` _asbp_character))
  (`self.K2_DestroyActor`))

(fn `Coin Spawn Points`
  (for _array_element (`self.Lane Position`)
    (for _index (range 201)
      (bind _returnvalue (`AddComponent|NODE_AddArrowComponent-0` :`RelativeTransform` (`KismetMathLibrary.MakeTransform` (`KismetMathLibrary.MakeVector` _array_element (* _index -425.0) 900.0))))
      (`ArrowComponent.SetArrowColor` _returnvalue (struct :`R` 1.0 :`G` 0.997723 :`B` 0.858276 :`A` 1.0))
      (`KismetArrayLibrary.Array_Add` (`self.CSpawn Points`) (`SceneComponent.K2_GetComponentToWorld` _returnvalue)))))

(fn `Get Attach Point Hallway`
  (returns (ReturnValue :type "Transform Structure"))
  (return (`SceneComponent.K2_GetComponentToWorld` (`self.Arrow`))))

(fn `SpawnCoins`
  (locals (`Random Spawn Points` :type "Array of Transform Structure"))
  (bind _output_get (set `local.Random Spawn Points` (`self.CSpawn Points`)))
  (`KismetArrayLibrary.Array_Shuffle` _output_get)
  (for _index (range (+ (`KismetMathLibrary.RandomIntegerInRange` 50 150) 1))
    (switch `int` 0
      (:`0`
        (`AddComponent|NODE_AddChildActorComponent-1` :`RelativeTransform` (`KismetMathLibrary.MakeRelativeTransform` (`|GetArrayItem` (`local.Random Spawn Points`) _index) (`self.GetTransform`)))))))

(fn `UserConstructionScript`
  (`self.Coin Spawn Points`)
  (`self.SpawnCoins`))